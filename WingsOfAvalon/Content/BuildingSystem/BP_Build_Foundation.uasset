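; Building-system foundation piece that extends itself downward to reach the ground below it.
; On BeginPlay it line-traces down from four arrow components, up to 800 units each with debug drawing, and keeps the longest hit distance.
; It stacks static mesh extensions below itself at 200-unit steps to cover that distance, then applies a wood trimsheet material to them.
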(event `self.ReceiveBeginPlay`
  (`self.DistanceFromGround`))

(fn `DistanceFromGround`
  (locals (localDistance :type "Float (single-precision)" :default 0.0))
  (bind _output (`|GetArrayItem` (`self.Extentions`)))
  (bind (_distance _didhit) (`self.Trace` (`self.Arrow1`)))
  (if _didhit
    (set `local.localDistance` _distance))
  (bind (_distance_2 _didhit_2) (`self.Trace` (`self.Arrow2`)))
  (if (and _didhit_2 (> _distance_2 (`local.localDistance`)))
    (set `local.localDistance` _distance_2))
  (bind (_distance_3 _didhit_3) (`self.Trace` (`self.Arrow3`)))
  (if (and _didhit_3 (> _distance_3 (`local.localDistance`)))
    (set `local.localDistance` _distance_3))
  (bind (_distance_4 _didhit_4) (`self.Trace` (`self.Arrow4`)))
  (if (and _didhit_4 (> _distance_4 (`local.localDistance`)))
    (set `local.localDistance` _distance_4))
  (for _index (range 1 (+ (`KismetMathLibrary.Round` (/ (`local.localDistance`) 200.0)) 1))
    (bind _returnvalue (`AddComponent|NODE_AddStaticMeshComponent-0` :`RelativeTransform` (`KismetMathLibrary.MakeTransform` (* (0.0 0.0 -200.0) _index))))
    (`KismetArrayLibrary.Array_Add` (`self.Extentions`) _returnvalue))
  (`/Engine/EditorBlueprintResources/StandardMacros.IsValid` _output
    (:`Is Valid`
      (bind _output_get (set `self.FoundationMaterials` (`MeshComponent.GetMaterials` _output)))
      (for _array_element (`self.Extentions`)
        (for (_ _array_index) _output_get
          (`PrimitiveComponent.SetMaterial` _array_element _array_index "/Game/BuildingSystem/Materials/M_WoodTrimsheet.M_WoodTrimsheet"))))))

(fn `Trace`
  (params (Component :type "PrimitiveComponent Object Reference"))
  (returns (Distance :type "Float (single-precision)") (DidHit :type Boolean))
  (bind _returnvalue (`SceneComponent.K2_GetComponentLocation` Component))
  (bind (_outhit _returnvalue_2) (`KismetSystemLibrary.LineTraceSingle` :`Start` _returnvalue :`End` (- _returnvalue (0.0 0.0 800.0)) :`TraceChannel` "TraceTypeQuery1" :`DrawDebugType` "ForDuration"))
  (return (`.Distance` (`GameplayStatics.BreakHitResult` _outhit)) _returnvalue_2))

(fn `UserConstructionScript`
  (`parent.UserConstructionScript`))