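; BP_Build_Master is a base building-piece actor, apparently for placeable structures that are built with resources.
; SetMesh assigns the mesh, stores its materials and covers every slot with a wood trimsheet material, while SetBuildCost stores the resource cost.
; Helper functions return the box components and a default build ID of zero.
; InteractwithBuild is empty; the resource counting, material restore and collision switching logic is disconnected and never runs.
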(event `/Game/BuildingSystem/BPC_BuildInterface.SetMesh`
  (params (Mesh :type "StaticMesh Object Reference"))
  (bind _returnvalue (`MeshComponent.GetMaterials` (`self.Build Mesh`)))
  (`StaticMeshComponent.SetStaticMesh` (`self.Build Mesh`) Mesh)
  (set `self.Materials` _returnvalue)
  (for (_ _array_index) _returnvalue
    (`PrimitiveComponent.SetMaterial` (`self.Build Mesh`) _array_index "/Game/BuildingSystem/Materials/M_WoodTrimsheet.M_WoodTrimsheet")))

(event `/Game/BuildingSystem/BPC_BuildInterface.SetBuildCost`
  (params (Resources :type Integer))
  (set `self.Cost` Resources))

(event `/Game/BuildingSystem/BPC_BuildInterface.InteractwithBuild`)

(fn `BuildID`
  (returns (NewParam :type Integer))
  (return 0))

(fn `Return Boxes`
  (returns (Boxes :type "Array of BoxComponent Object Reference"))
  (return (`self.K2_GetComponentsByClass` "/Script/Engine.BoxComponent")))

(fn `UserConstructionScript`)