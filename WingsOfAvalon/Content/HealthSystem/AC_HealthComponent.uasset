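; Actor component that tracks an owner's health through AddHealth and RemoveHealth events.
; AddHealth's select is inverted relative to a cap: it sets MaxHealth when the sum is below it, otherwise keeps the sum.
; RemoveHealth floors health at zero, then calls DeathMessage on the owner if the already-updated health minus the damage is zero or less.
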(event `/Game/HealthSystem/BI_HealthInterface.AddHealth`
  (params (Health :type "Float (double-precision)"))
  (bind _maxhealth (`self.MaxHealth`))
  (bind _returnvalue (+ Health (`self.CurrentHealth`)))
  (set `self.CurrentHealth` (`KismetMathLibrary.SelectFloat` _maxhealth _returnvalue (< _returnvalue _maxhealth))))

(event `/Game/HealthSystem/BI_HealthInterface.RemoveHealth`
  (params (Health :type "Float (double-precision)"))
  (bind _returnvalue (- (`self.CurrentHealth`) Health))
  (bind _returnvalue_2 (<= _returnvalue 0.0))
  (set `self.CurrentHealth` (`KismetMathLibrary.SelectFloat` 0.0 _returnvalue _returnvalue_2))
  (if _returnvalue_2
    (message `/Game/HealthSystem/BI_Death.Death` (`self.GetOwner`))))