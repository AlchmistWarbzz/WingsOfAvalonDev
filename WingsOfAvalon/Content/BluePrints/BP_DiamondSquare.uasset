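; BP_DiamondSquare builds a flat procedural grid mesh at BeginPlay; despite its name, it contains no diamond-square height displacement.
; CreateVertices fills a scaled XSize by YSize vertex grid at zero height with matching UVs, while CreateTriangles indexes only the first quad.
; The ProceduralMesh section is created with collision and a material, then long-lived debug spheres are drawn using vertex positions.
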(event `self.ReceiveBeginPlay`
  (bind _vertices (`self.Vertices`))
  (`self.CreateVertices`)
  (`self.Create Triangles`)
  (`ProceduralMeshComponent.CreateMeshSection_LinearColor` :`self` (`self.ProceduralMesh`) :`Vertices` _vertices :`Triangles` (`self.Triangles`) :`UV0` (`self.UV0`) :`bCreateCollision` true)
  (`PrimitiveComponent.SetMaterial` (`self.ProceduralMesh`) 0 (`self.Material`))
  (for _array_element _vertices
    (`KismetSystemLibrary.DrawDebugSphere` (`KismetMathLibrary.MakeVector` (.x _array_element) (.y _array_element)) 25.0 12 (struct :`R` 1.0 :`G` 0.006821 :`A` 1.0) 999.0)))

(fn `Create Triangles`
  (`KismetArrayLibrary.Array_Add` (`self.Triangles`))
  (`KismetArrayLibrary.Array_Add` (`self.Triangles`) 1)
  (`KismetArrayLibrary.Array_Add` (`self.Triangles`) (+ (`self.YSize`) 1))
  (`KismetArrayLibrary.Array_Add` (`self.Triangles`) 1)
  (`KismetArrayLibrary.Array_Add` (`self.Triangles`) (+ (`self.YSize`) 2))
  (`KismetArrayLibrary.Array_Add` (`self.Triangles`) (+ (`self.YSize`) 1)))

(fn `CreateVertices`
  (locals (X :type Integer) (Y :type Integer))
  (for _index (range (+ (`self.XSize`) 1))
    (set `local.X` _index)
    (for _index_2 (range (+ (`self.YSize`) 1))
      (set `local.Y` _index_2)
      (`KismetArrayLibrary.Array_Add` (`self.Vertices`) (`KismetMathLibrary.MakeVector` (* (`local.X`) (`self.Scale`)) (* (`local.Y`) (`self.Scale`))))
      (`KismetArrayLibrary.Array_Add` (`self.UV0`) (`KismetMathLibrary.MakeVector2D` (* (`local.X`) (`self.UVScale`)) (* (`local.Y`) (`self.UVScale`)))))))

(fn `UserConstructionScript`)